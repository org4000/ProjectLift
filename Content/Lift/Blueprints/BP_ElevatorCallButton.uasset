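; Elevator call button actor that creates a call button mesh for a given floor through its SpawnButton event.
; SpawnButton adds a static mesh component at runtime, placing it from CallButtonStartPos with depth and horizontal offsets.
; Each button is tagged as ElevatorCallButton plus its floor value, so it can be identified by tag.
; CallButtonHeight grows by the elevator's FloorHeight per spawn but does not affect the button's position.
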(event `SpawnButton`
  (params (FloorValue :type Name))
  ;[1 1 1] Comment
  (set `self.Floor Value` FloorValue)
  (bind _returnvalue (`AddComponent|NODE_AddStaticMeshComponent-0` :`RelativeTransform` (`SceneComponent.GetRelativeTransform` (`self.CallButtonStartPos`))))
  (`StaticMeshComponent.SetStaticMesh` _returnvalue (`self.CallButtonMesh`))
  (set `self.CallButtonRef` _returnvalue)
  ;[1 1 1] Comment
  (`SceneComponent.K2_SetRelativeLocation` (`self.CallButtonRef`) (`KismetMathLibrary.MakeVector` (- (.x (.location (`SceneComponent.GetRelativeTransform` (`self.CallButtonStartPos`)))) (`self.CallButtonDepthOffset`)) (- (.y (.location (`SceneComponent.GetRelativeTransform` (`self.CallButtonStartPos`)))) (`self.CallButtonHorOffset`)) (.z (.location (`SceneComponent.GetRelativeTransform` (`self.CallButtonStartPos`))))) false false)
  (set `ActorComponent.ComponentTags` (`|MakeArray` "ElevatorCallButton" (`self.Floor Value`)) (`self.CallButtonRef`))
  (set `self.CallButtonHeight` (+ (`self.CallButtonHeight`) (`/Game/Lift/Blueprints/BP_Cabin.FloorHeight` (`self.ElevatorRef`)))))

(fn `UserConstructionScript`)