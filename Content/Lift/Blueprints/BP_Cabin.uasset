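; Elevator cabin actor that spawns its call button and an attached floor-button control panel on BeginPlay, passing each a reference to itself.
; GoToFloorEvent ignores requests while moving, otherwise runs the door timeline, waits, then starts ElevatorUp or ElevatorDown.
; Both share one timeline lerping Z to floor times height, with play rate scaled by target floor going up and floor difference going down.
; Doors animate through X scale.
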(event `self.ReceiveBeginPlay`
  (bind _returnvalue_location (`KismetMathLibrary.BreakTransform` (`SceneComponent.K2_GetComponentToWorld` (`self.ButtonArrow`))))
  (bind (_returnvalue_x _returnvalue_y _returnvalue_z) (`KismetMathLibrary.BreakVector` (`SceneComponent.K2_GetComponentLocation` (`self.ControlPanelArrow`))))
  ;[1 1 1] Comment
  (bind _returnvalue (`|SpawnActorFromClass` "/Game/Lift/Blueprints/BP_ElevatorCallButton.BP_ElevatorCallButton_C" (`KismetMathLibrary.MakeTransform` _returnvalue_location) "Undefined" "MultiplyWithRoot" null (`self.Call Button Vert Offset`) (`self.Call Button Hor Offset`) (`self.Call Button Depth Offset`) (`self.Call Button Mesh`) self null))
  (set `self.ElevatorCallButtonRef` _returnvalue)
  (bind _returnvalue_2 (`|SpawnActorFromClass` "/Game/Lift/Blueprints/BP_ControlPanel.BP_ControlPanel_C" (`KismetMathLibrary.MakeTransform` (`KismetMathLibrary.MakeVector` (+ _returnvalue_x (`self.Call Button Depth Offset`)) (+ _returnvalue_y (`self.ControlPanelHorOffset`)) (+ _returnvalue_z (`self.ControlPanelVertOffset`)))) "Undefined" "MultiplyWithRoot" null (`self.Control Panel Button Offset`) (`self.Max Horizontal Buttons`) (`self.Number Of Floors`) (`self.Control Panel Button Distance Between Hor`) (`self.Control Panel Button Distance Between Vert`) self null))
  (`self.K2_AttachToActor` _returnvalue_2 self "None" "KeepWorld" "KeepWorld" "KeepWorld" true))

(event `ElevatorUp`
  (bind (_returnvalue_x _returnvalue_y _returnvalue_z) (`KismetMathLibrary.BreakVector` (`self.K2_GetActorLocation`)))
  (bind (_returnvalue_x_2 _returnvalue_y_2) (`KismetMathLibrary.BreakVector` (`self.K2_GetActorLocation`)))
  (bind (_returnvalue_x_3 _returnvalue_y_3 _returnvalue_z_2) (`KismetMathLibrary.BreakVector` (`self.K2_GetActorLocation`)))
  (`TimelineComponent.SetPlayRate` (`self.GoingUpDownTimeline`) (/ (/ 1.0 (`self.ElevatorSpeed`)) (`self.FloorToRef`)))
  (set `self.StartZ` _returnvalue_z_2 :!label _label)
  (bind (_direction _goingupdowntimelinenewtrack) (`Timeline|GoingUpDownTimeline` :!via `PlayFromStart`)
    (:`Update`
      (`self.K2_SetActorLocation` (`KismetMathLibrary.MakeVector` _returnvalue_x_2 _returnvalue_y_2 (`KismetMathLibrary.Lerp` (`self.StartZ`) (`KismetMathLibrary.Conv_IntToDouble` (* (`self.FloorToRef`) (`KismetMathLibrary.FTrunc` (`self.FloorHeight`)))) _goingupdowntimelinenewtrack))))
    (:`Finished`
      (set `self.StartZ` _returnvalue_z)
      (set `self.WhatFloorWeAt?` (`self.FloorToRef`))
      (`self.OpenCloseElevatorDoors` false)
      (`KismetSystemLibrary.Delay` (`TimelineComponent.GetPlayRate` (`self.OpenCloseElevatorDoorsTimeline`)))
      (set `self.CurrentlyActive?` false))))

(event `GoToFloorEvent`
  (params (Floor :type Integer))
  ;[1 1 1] Comment
  (if (not (`self.CurrentlyActive?`))
    (set `self.FloorToRef` Floor)
    (if (== (`self.FloorToRef`) (`self.WhatFloorWeAt?`))
      (`KismetSystemLibrary.PrintString` (`KismetStringLibrary.Concat_StrStr` "Already at floor " (`KismetStringLibrary.Conv_IntToString` (`self.FloorToRef`)) "" "Opening door "))
      (`self.OpenCloseElevatorDoors` true)
      (else
        (set `self.CurrentlyActive?` true)
        (`KismetSystemLibrary.PrintString` (`KismetStringLibrary.Concat_StrStr` "Going to floor " (`KismetStringLibrary.Conv_IntToString` (`self.FloorToRef`)) "" "Closing the doors"))
        (`self.OpenCloseElevatorDoors` false)
        (`KismetSystemLibrary.Delay` (`TimelineComponent.GetPlayRate` (`self.OpenCloseElevatorDoorsTimeline`)))
        (if (> (`self.FloorToRef`) (`self.WhatFloorWeAt?`))
          (`self.ElevatorUp`)
          (else
            (`self.ElevatorDown`)))))))

(event `ElevatorDown`
  (`TimelineComponent.SetPlayRate` (`self.GoingUpDownTimeline`) (/ (/ 1.0 (`self.ElevatorSpeed`)) (`KismetMathLibrary.Conv_IntToDouble` (- (`self.WhatFloorWeAt?`) (`self.FloorToRef`)))))
  (goto _label))

(event `OpenCloseElevatorDoors`
  (params (`Open?` :type Boolean))
  (bind (_relativescale3d_x _relativescale3d_y _relativescale3d_z) (`KismetMathLibrary.BreakVector` (`SceneComponent.RelativeScale3D` (`self.Door1`))))
  ;[1 1 1] Comment
  (`TimelineComponent.SetPlayRate` (`self.OpenCloseElevatorDoorsTimeline`) (/ 1.0 (`self.ElevatorDoorsSpeed`)))
  (if `Open?`
    (bind (_direction _opencloseelevatordoorsnewtrack) (`Timeline|OpenCloseElevatorDoorsTimeline` :!via `PlayFromStart` :!label _label_2)
      (:`Update`
        (`SceneComponent.SetRelativeScale3D` (`self.Door0`) (`KismetMathLibrary.MakeVector` (`KismetMathLibrary.Lerp` 0.0 0.1 _opencloseelevatordoorsnewtrack) _relativescale3d_y _relativescale3d_z))
        (`SceneComponent.SetRelativeScale3D` (`self.Door1`) (`KismetMathLibrary.MakeVector` (`KismetMathLibrary.Lerp` 0.0 0.1 _opencloseelevatordoorsnewtrack) _relativescale3d_y _relativescale3d_z))))
    (else
      (goto _label_2 :!via `ReverseFromEnd`))))

(fn `UserConstructionScript`)